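; Breakable maze pillar that drops either a key (BP_Chave) or an enemy, depending on HasKey, which its text render displays every tick.
; Overlaps from a BP_PlayerPawn with Stop set destroy the physics constraint; the Collider also triggers BaterNaArvore.
; A server hit event spawns the content once when the cube strikes a "Chao"-tagged actor, then removes the cube after a delay.
; Player hits on the pillar apply a GAS slowdown on authority, and Chaos breaks add force.
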(event `self.ReceiveTick`
  (params (DeltaSeconds :type "Float (single-precision)"))
  (`TextRenderComponent.K2_SetText` (`self.TextRender`) (`KismetTextLibrary.Conv_BoolToText` (`self.HasKey`))))

(event `self.Pilar.OnComponentBeginOverlap`
  (params (OverlappedComponent :type "PrimitiveComponent Object Reference") (OtherActor :type "Actor Object Reference") (OtherComp :type "PrimitiveComponent Object Reference") (OtherBodyIndex :type Integer) (bFromSweep :type Boolean) (SweepResult :type "HitResult Structure (by ref)"))
  (bind _asbp_player_pawn (cast `/Game/AlvesCostaMaze/BP_PlayerPawn` OtherActor))
  (if (`/Game/AlvesCostaMaze/BP_PlayerPawn.bStop` _asbp_player_pawn)
    (`ActorComponent.K2_DestroyComponent` (`self.PhysicsConstraint`))))

(event `self.Collider.OnComponentBeginOverlap`
  (params (OverlappedComponent :type "PrimitiveComponent Object Reference") (OtherActor :type "Actor Object Reference") (OtherComp :type "PrimitiveComponent Object Reference") (OtherBodyIndex :type Integer) (bFromSweep :type Boolean) (SweepResult :type "HitResult Structure (by ref)"))
  (bind _asbp_player_pawn (cast `/Game/AlvesCostaMaze/BP_PlayerPawn` OtherActor))
  (if (`/Game/AlvesCostaMaze/BP_PlayerPawn.bStop` _asbp_player_pawn)
    (`/Game/AlvesCostaMaze/BP_PlayerPawn.Bater na Arvore` _asbp_player_pawn)
    (`ActorComponent.K2_DestroyComponent` (`self.PhysicsConstraint`))))

(event `self.Cube.OnComponentHit`
  (params (HitComponent :type "PrimitiveComponent Object Reference") (OtherActor :type "Actor Object Reference") (OtherComp :type "PrimitiveComponent Object Reference") (NormalImpulse :type "Vector Structure") (Hit :type "HitResult Structure (by ref)"))
  (`self.Server_HitPillar` OtherActor))

(event `Server_HitPillar`
  (params (ActorHit :type "Actor Object Reference"))
  (if (`self.ActorHasTag` ActorHit "Chao")
    (if (not (`self.bHasSpawned`))
      (set `self.bHasSpawned` true)
      (if (`self.HasKey`)
        (`|SpawnActorFromClass` "/Game/AlvesCostaMaze/BP_Chave.BP_Chave_C" (`KismetMathLibrary.Conv_VectorToTransform` (`.ImpactPoint` (`GameplayStatics.BreakHitResult` (stale `self.Cube.OnComponentHit` Hit)))) "Undefined" "MultiplyWithRoot" null null)
        (else
          (`|SpawnActorFromClass` "/Game/AlvesCostaMaze/BP_Enemy.BP_Enemy_C" (`KismetMathLibrary.Conv_VectorToTransform` (`.ImpactPoint` (`GameplayStatics.BreakHitResult` (stale `self.Cube.OnComponentHit` Hit)))) "Undefined" "MultiplyWithRoot" null null)))
      (`KismetSystemLibrary.Delay` 6.0)
      (`ActorComponent.K2_DestroyComponent` (`self.Cube`)))))

(event `self.Cube.OnChaosBreakEvent`
  (params (BreakEvent :type "ChaosBreakEvent Structure (by ref)"))
  (bind _returnvalue (`AddComponent|NODE_AddRadialFalloff-1`))
  (`GeometryCollectionComponent.ApplyPhysicsField` (`self.Cube`) false "Chaos_LinearForce" null _returnvalue))

(event `self.Pilar.OnComponentHit`
  (params (HitComponent :type "PrimitiveComponent Object Reference") (OtherActor :type "Actor Object Reference") (OtherComp :type "PrimitiveComponent Object Reference") (NormalImpulse :type "Vector Structure") (Hit :type "HitResult Structure (by ref)"))
  (`/Engine/EditorBlueprintResources/ActorMacros.Switch Has Authority`
    (:`Authority`
      (bind _asbp_player_pawn (cast `/Game/AlvesCostaMaze/BP_PlayerPawn` OtherActor))
      (`/Engine/EditorBlueprintResources/StandardMacros.DoOnce` false :!label _label
        (:`Completed`
          (`PrimitiveComponent.SetSimulatePhysics` (`/Game/AlvesCostaMaze/BP_PlayerPawn.Capsule` _asbp_player_pawn) false)
          (`AbilitySystemComponent.BP_ApplyGameplayEffectToSelf` :`self` (`AbilitySystemBlueprintLibrary.GetAbilitySystemComponent` OtherActor) :`GameplayEffectClass` "/Game/AlvesCostaMaze/GAS/GA_Lentidao.GA_Lentidao_C")
          (`PrimitiveComponent.SetSimulatePhysics` (`/Game/AlvesCostaMaze/BP_PlayerPawn.Capsule` _asbp_player_pawn) true)
          (`KismetSystemLibrary.Delay` 0.12)
          (goto _label :!via `Reset`))))))

(fn `NewFunction`)

(fn `OnRep_bHasSpawned`)

(fn `OnRep_HasKey`)

(fn `UserConstructionScript`)