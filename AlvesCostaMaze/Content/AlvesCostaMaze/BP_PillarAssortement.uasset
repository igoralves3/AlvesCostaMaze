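; BP_PillarAssortement is a level actor that randomly picks which maze pillar holds the key when play begins.
; On BeginPlay it gathers every BP_Pilar in the world, shuffles the array and sets HasKey on the first one.
; It also prints each pillar to the screen as it loops through them.
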(event `self.ReceiveBeginPlay`
  (bind _outactors (`GameplayStatics.GetAllActorsOfClass` "/Game/AlvesCostaMaze/BP_Pilar.BP_Pilar_C"))
  (bind _output_get (set `self.Out Actors` _outactors))
  (`KismetArrayLibrary.Array_Shuffle` _output_get)
  (for (_array_element _array_index) (`self.Out Actors`)
    (`KismetSystemLibrary.PrintText` (`KismetTextLibrary.Conv_ObjectToText` _array_element))
    (if (<= _array_index 0)
      (bind _asbp_pilar (cast `/Game/AlvesCostaMaze/BP_Pilar` _array_element))
      (set `/Game/AlvesCostaMaze/BP_Pilar.HasKey` true _asbp_pilar))))

(fn `UserConstructionScript`)