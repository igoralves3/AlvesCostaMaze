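; Maze enemy character that targets the nearest BP_PlayerPawn, turns its cylinder toward it and lunges when close.
; Tick triggers the horizontal launch with a speed boost and velocity-scaled Niagara trail, using a delay as cooldown.
; RunToPlay loops AIMoveTo, but BeginPlay calls it before a target is set, so it only runs the search.
; Server-side capsule hits apply GA_Dano damage through GAS, throttled by a resetting DoOnce.
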(event `self.ReceiveBeginPlay`
  (`self.RunToPlay`)
  (`self.NearestPlayer`))

(event `NearestPlayer`
  (bind _outactors (`GameplayStatics.GetAllActorsOfClass` "/Game/AlvesCostaMaze/BP_PlayerPawn.BP_PlayerPawn_C"))
  (bind (_distance _returnvalue) (`GameplayStatics.FindNearestActor` (`self.K2_GetActorLocation`) _outactors))
  (`/Engine/EditorBlueprintResources/StandardMacros.IsValid` _returnvalue
    (:`Is Valid`
      (bind _asbp_player_pawn (cast `/Game/AlvesCostaMaze/BP_PlayerPawn` _returnvalue))
      (set `self.Current Player` _asbp_player_pawn))))

(event `self.ReceiveActorBeginOverlap`
  (params (OtherActor :type "Actor Object Reference"))
  (cast `/Game/AlvesCostaMaze/BP_PlayerPawn` OtherActor))

(event `self.ReceiveTick`
  (params (DeltaSeconds :type "Float (single-precision)"))
  (bind _returnvalue (- (`self.K2_GetActorLocation` (`self.Current Player`)) (`self.K2_GetActorLocation`)))
  (`SceneComponent.K2_SetWorldRotation` (`self.Cylinder`) (`KismetMathLibrary.FindLookAtRotation` (`SceneComponent.K2_GetComponentLocation` (`self.Cylinder`)) (`self.K2_GetActorLocation` (`self.Current Player`))) false false)
  (if (`self.canImpulse`)
    (if (< (`KismetMathLibrary.VSize` _returnvalue) 1000.0)
      (if (`self.canImpulse`)
        (set `self.canImpulse` false)
        (`NiagaraComponent.SetNiagaraVariableInt` (`self.Ghots_Trial`) "Spawn Count" (`KismetMathLibrary.FTrunc` (* (`KismetMathLibrary.VSize` (`MovementComponent.Velocity` (`self.CharacterMovement`))) 5.0)))
        (set `CharacterMovementComponent.MaxWalkSpeed` 1500.0 (`self.CharacterMovement`))
        (`self.LaunchCharacter` (* (`KismetMathLibrary.Normal` _returnvalue) (1500.0 1500.0 0.0)) true)
        (`KismetSystemLibrary.PrintString` "enemy attack")))
    (else
      (`KismetSystemLibrary.Delay` 1.0)
      (set `self.canImpulse` true)
      (set `CharacterMovementComponent.MaxWalkSpeed` 200.0 (`self.CharacterMovement`)))))

(event `RunToPlay`
  (`/Engine/EditorBlueprintResources/StandardMacros.IsValid` (`self.Current Player`)
    (:`Is Valid`
      (`|AIMoveTo` self (`self.K2_GetActorLocation` (`self.Current Player`)) (`self.Current Player`) 5.0 true
        (:`OnSuccess`
          (`KismetSystemLibrary.Delay` 1.0))
        (:`OnFail`
          _))
      (`self.RunToPlay`))
    (:`Is Not Valid`
      (`self.NearestPlayer`))))

(event `self.Sphere.OnComponentHit`
  (params (HitComponent :type "PrimitiveComponent Object Reference") (OtherActor :type "Actor Object Reference") (OtherComp :type "PrimitiveComponent Object Reference") (NormalImpulse :type "Vector Structure") (Hit :type "HitResult Structure (by ref)")))

(event `self.CapsuleComponent.OnComponentHit`
  (params (HitComponent :type "PrimitiveComponent Object Reference") (OtherActor :type "Actor Object Reference") (OtherComp :type "PrimitiveComponent Object Reference") (NormalImpulse :type "Vector Structure") (Hit :type "HitResult Structure (by ref)"))
  (`/Engine/EditorBlueprintResources/ActorMacros.Switch Has Authority`
    (:`Authority`
      (bind _asbp_player_pawn (cast `/Game/AlvesCostaMaze/BP_PlayerPawn` OtherActor))
      (`/Engine/EditorBlueprintResources/StandardMacros.DoOnce` false :!label _label
        (:`Completed`
          (`PrimitiveComponent.SetSimulatePhysics` (`/Game/AlvesCostaMaze/BP_PlayerPawn.Capsule` _asbp_player_pawn) false)
          (`AbilitySystemComponent.BP_ApplyGameplayEffectToSelf` :`self` (`AbilitySystemBlueprintLibrary.GetAbilitySystemComponent` OtherActor) :`GameplayEffectClass` "/Game/AlvesCostaMaze/GAS/GA_Dano.GA_Dano_C")
          (`PrimitiveComponent.SetSimulatePhysics` (`/Game/AlvesCostaMaze/BP_PlayerPawn.Capsule` _asbp_player_pawn) true)
          (`KismetSystemLibrary.Delay` 0.5)
          (goto _label :!via `Reset`))))))

(fn `UserConstructionScript`)