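; Player pawn for a maze game, with control-yaw-relative floating movement and a chargeable spin dash.
; Holding left mouse disables movement and builds charge on Tick; release launches the physics capsule forward, restoring movement a second later.
; Overlapping a BP_Door stores it so E can trigger it; the overlap flag is never cleared.
; It creates the HUD, whose key text UpdateHUD sets; manual jump logic is disconnected.
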(event `self.ReceiveBeginPlay`
  (`ActorComponent.Activate` (`self.FloatingPawnMovement`) false)
  (`PrimitiveComponent.SetSimulatePhysics` (`self.Capsule`) true)
  (set `self.Keys` 0)
  (bind _returnvalue (`|CreateWidget` "/Game/AlvesCostaMaze/HUD/BP_HUD.BP_HUD_C"))
  (bind _output_get (set `self.HUD` _returnvalue))
  (`UserWidget.AddToViewport` _output_get 0))

(event `InputAxis|Turn`
  (params (AxisValue :type "Float (single-precision)"))
  (`self.AddControllerYawInput` AxisValue))

(event `InputAxis|LookUp`
  (params (AxisValue :type "Float (single-precision)"))
  (`self.AddControllerPitchInput` AxisValue))

(event `InputAxis|MoveRight`
  (params (AxisValue :type "Float (single-precision)"))
  (`self.AddMovementInput` (`KismetMathLibrary.GetRightVector` (`KismetMathLibrary.MakeRotator` 0.0 0.0 (.yaw (`self.GetControlRotation`)))) AxisValue))

(event `InputAxis|MoveForward`
  (params (AxisValue :type "Float (single-precision)"))
  (`self.AddMovementInput` (`KismetMathLibrary.GetForwardVector` (`KismetMathLibrary.MakeRotator` 0.0 0.0 (.yaw (`self.GetControlRotation`)))) AxisValue))

(event `InputAction|Jump`
  (params (Key :type "Key Structure")))

(event `self.ReceiveTick`
  (params (DeltaSeconds :type "Float (single-precision)"))
  (if (`self.bSpinDash?`)
    (bind _output_get (set `self.fCharge` (`KismetMathLibrary.FClamp` (+ (* DeltaSeconds (`self.fChargeRate`)) (`self.fCharge`)) 0.0 (`self.fFloatChargeMax`))))))

(event `Key|LeftMouseButton`
  (params (Key :type "Key Structure"))
  ; SpinDash
  (:`Pressed`
    (set `self.bStop` true)
    (`ActorComponent.Deactivate` (`self.FloatingPawnMovement`))
    (`PrimitiveComponent.SetSimulatePhysics` (`self.Capsule`) true)
    (set `self.bSpinDash?` true)
    (set `self.fCharge` 0.0))
  (:`Released`
    (set `self.bSpinDash?` false)
    (`PrimitiveComponent.SetSimulatePhysics` (`self.Capsule`) true)
    (`PrimitiveComponent.AddImpulse` (`self.Capsule`) (* (`KismetMathLibrary.GetForwardVector` (`KismetMathLibrary.MakeRotator` 0.0 0.0 (.yaw (`self.GetControlRotation`)))) (`self.fCharge`)) "None" true)
    (`KismetSystemLibrary.Delay` 1.0)
    (`ActorComponent.Activate` (`self.FloatingPawnMovement`) false)
    (`PrimitiveComponent.SetSimulatePhysics` (`self.Capsule`) false)
    (set `self.bStop` false)))

(event `self.Capsule.OnComponentHit`
  (params (HitComponent :type "PrimitiveComponent Object Reference") (OtherActor :type "Actor Object Reference") (OtherComp :type "PrimitiveComponent Object Reference") (NormalImpulse :type "Vector Structure") (Hit :type "HitResult Structure (by ref)")))

(event `self.Capsule.OnComponentBeginOverlap`
  (params (OverlappedComponent :type "PrimitiveComponent Object Reference") (OtherActor :type "Actor Object Reference") (OtherComp :type "PrimitiveComponent Object Reference") (OtherBodyIndex :type Integer) (bFromSweep :type Boolean) (SweepResult :type "HitResult Structure (by ref)"))
  (bind _asbp_door (cast `/Game/AlvesCostaMaze/BP_Door` OtherActor))
  (set `self.bApertou?` true)
  (set `self.Porta` _asbp_door))

(event `Key|E`
  (params (Key :type "Key Structure"))
  ; Interação_com_a_porta
  (:`Pressed`
    (if (`self.bApertou?`)
      (set `/Game/AlvesCostaMaze/BP_Door.JogarInteragiu` true (`self.Porta`)))))

(event `Update HUD`
  (`TextBlock.SetText` (`/Game/AlvesCostaMaze/HUD/BP_HUD.Text_Keys` (`self.HUD`)) (`|FormatText` "Keys: {Keys}" (`self.Valor`))))

(fn `UserConstructionScript`)