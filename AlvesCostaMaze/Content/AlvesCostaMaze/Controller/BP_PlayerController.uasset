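; Player controller for the maze game that relays Enhanced Input actions to its PlayerPawn reference.
; Move and turn inputs go to the pawn's Server-prefixed events, while the open input calls AbrePorta (open door), each guarded by a validity check.
; BeginPlay hides the mouse cursor.
; ClientSpawnPawn spawns a BP_PlayerPawn at the controller's transform without possessing it or setting PlayerPawn here, and trocaFase (change stage) is an empty stub.
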(event `EnhancedInput|/Game/AlvesCostaMaze/InputMap/IA_MoveForward`
  (params (ActionValue :type "Float (double-precision)") (ElapsedSeconds :type "Float (double-precision)") (TriggeredSeconds :type "Float (double-precision)") (InputAction :type "InputAction Object Reference" :default "/Game/AlvesCostaMaze/InputMap/IA_MoveForward.IA_MoveForward"))
  (bind _player_pawn (`self.Player Pawn`))
  (:`Triggered`
    (`/Engine/EditorBlueprintResources/StandardMacros.IsValid` _player_pawn
      (:`Is Valid`
        (`/Game/AlvesCostaMaze/BP_PlayerPawn.Server  MoveForward` _player_pawn ActionValue)))))

(event `self.ReceiveBeginPlay`
  (set `PlayerController.bShowMouseCursor` false (`GameplayStatics.GetPlayerController` 0)))

(event `EnhancedInput|/Game/AlvesCostaMaze/InputMap/IA_MoveRight`
  (params (ActionValue :type "Float (double-precision)") (ElapsedSeconds :type "Float (double-precision)") (TriggeredSeconds :type "Float (double-precision)") (InputAction :type "InputAction Object Reference" :default "/Game/AlvesCostaMaze/InputMap/IA_MoveRight.IA_MoveRight"))
  (bind _player_pawn (`self.Player Pawn`))
  (:`Triggered`
    (`/Engine/EditorBlueprintResources/StandardMacros.IsValid` _player_pawn
      (:`Is Valid`
        (`/Game/AlvesCostaMaze/BP_PlayerPawn.Server Move Right` _player_pawn ActionValue)))))

(event `ClientSpawnPawn`
  (`|SpawnActorFromClass` "/Game/AlvesCostaMaze/BP_PlayerPawn.BP_PlayerPawn_C" (`self.GetTransform`) "Undefined" "MultiplyWithRoot" null null))

(event `EnhancedInput|/Game/AlvesCostaMaze/InputMap/IA_Turn`
  (params (ActionValue :type "Vector2D Structure") (ElapsedSeconds :type "Float (double-precision)") (TriggeredSeconds :type "Float (double-precision)") (InputAction :type "InputAction Object Reference" :default "/Game/AlvesCostaMaze/InputMap/IA_Turn.IA_Turn"))
  (bind _player_pawn (`self.Player Pawn`))
  (:`Triggered`
    (`/Engine/EditorBlueprintResources/StandardMacros.IsValid` _player_pawn
      (:`Is Valid`
        (`/Game/AlvesCostaMaze/BP_PlayerPawn.Server Turn` _player_pawn (`KismetMathLibrary.BreakVector2D` ActionValue))))))

(event `EnhancedInput|/Game/AlvesCostaMaze/InputMap/IA_Open`
  (params (ActionValue :type Boolean) (ElapsedSeconds :type "Float (double-precision)") (TriggeredSeconds :type "Float (double-precision)") (InputAction :type "InputAction Object Reference" :default "/Game/AlvesCostaMaze/InputMap/IA_Open.IA_Open"))
  (bind _player_pawn (`self.Player Pawn`))
  (:`Triggered`
    (`/Engine/EditorBlueprintResources/StandardMacros.IsValid` _player_pawn
      (:`Is Valid`
        (`/Game/AlvesCostaMaze/BP_PlayerPawn.AbrePorta` _player_pawn)))))

(event `trocaFase`)

(event `Key|E`
  (params (Key :type "Key Structure")))

(fn `UserConstructionScript`)