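; Maze platform with a trigger that applies gameplay effects to a player standing on it, handled only on the server.
; On overlap it starts the BP_PlayerPawn's particle effect and applies GA_Charge and GA_Lentidao (slowness) through the Ability System.
; Leaving removes only the charge effect via its saved handle and ends particles on the last stored player.
; End overlap has no pawn check, and one handle and player reference serve all overlaps.
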(event `self.Trigger.OnComponentBeginOverlap`
  (params (OverlappedComponent :type "PrimitiveComponent Object Reference") (OtherActor :type "Actor Object Reference") (OtherComp :type "PrimitiveComponent Object Reference") (OtherBodyIndex :type Integer) (bFromSweep :type Boolean) (SweepResult :type "HitResult Structure (by ref)"))
  (bind _returnvalue (`AbilitySystemBlueprintLibrary.GetAbilitySystemComponent` OtherActor))
  (`/Engine/EditorBlueprintResources/ActorMacros.Switch Has Authority`
    (:`Authority`
      (bind _asbp_player_pawn (cast `/Game/AlvesCostaMaze/BP_PlayerPawn` OtherActor))
      (set `self.Player` _asbp_player_pawn)
      (`/Game/AlvesCostaMaze/BP_PlayerPawn.Particula` _asbp_player_pawn)
      (bind _returnvalue_2 (`AbilitySystemComponent.BP_ApplyGameplayEffectToSelf` :`self` _returnvalue :`GameplayEffectClass` "/Game/AlvesCostaMaze/GAS/GA_Charge.GA_Charge_C"))
      (set `self.HandleDoEfeito` _returnvalue_2)
      (`AbilitySystemComponent.BP_ApplyGameplayEffectToSelf` :`self` _returnvalue :`GameplayEffectClass` "/Game/AlvesCostaMaze/GAS/GA_Lentidao.GA_Lentidao_C"))))

(event `self.Trigger.OnComponentEndOverlap`
  (params (OverlappedComponent :type "PrimitiveComponent Object Reference") (OtherActor :type "Actor Object Reference") (OtherComp :type "PrimitiveComponent Object Reference") (OtherBodyIndex :type Integer))
  (`/Engine/EditorBlueprintResources/ActorMacros.Switch Has Authority`
    (:`Authority`
      (`AbilitySystemComponent.RemoveActiveGameplayEffect` (`AbilitySystemBlueprintLibrary.GetAbilitySystemComponent` OtherActor) (`self.HandleDoEfeito`) -1)
      (`/Game/AlvesCostaMaze/BP_PlayerPawn.FimParticula` (`self.Player`)))))

(fn `UserConstructionScript`)