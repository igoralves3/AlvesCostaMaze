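; BP_Door is a maze exit door that swings open and changes level once the player has won.
; Tick waits for the player pawn's Venceu flag and the door's JogarInteragiu flag, then runs OpenDoor.
; A Timeline rotates the door mesh to 90° yaw, then LevelChange opens Level1 or Menu based on the current level name.
; Older overlap and key-count logic is disconnected, leaving KeysRequired only printed at BeginPlay.
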(event `self.ReceiveBeginPlay`
  (bind _output_get (set `self.KeysRequired` 1))
  (`KismetSystemLibrary.PrintString` (`KismetStringLibrary.Conv_IntToString` _output_get))
  (bind _outactors (`GameplayStatics.GetAllActorsOfClass` "/Game/AlvesCostaMaze/BP_PlayerPawn.BP_PlayerPawn_C"))
  (set `self.Player` (`|GetArrayItem` _outactors)))

(event `self.ReceiveTick`
  (params (DeltaSeconds :type "Float (single-precision)"))
  ; Jogador Aperta E abrir a porta
  (if (`/Game/AlvesCostaMaze/BP_PlayerPawn.bVenceu?` (`self.Player`))
    (if (`self.JogarInteragiu`)
      (set `self.canOpen` true)
      (`KismetSystemLibrary.PrintText` "door open")
      (`self.OpenDoor`))))

(event `LevelChange`
  (bind _returnvalue (`GameplayStatics.GetCurrentLevelName` true))
  (switch `string` _returnvalue
    (:`Default`
      (`GameplayStatics.OpenLevelBySoftObjectPtr` "/Game/AlvesCostaMaze/Levels/Menu.Menu" :!label _label))
    (:`Level1`
      (`GameplayStatics.OpenLevel` "Level1"))
    (:`Level2`
      (goto _label))))

(event `self.Collision.OnComponentBeginOverlap`
  (params (OverlappedComponent :type "PrimitiveComponent Object Reference") (OtherActor :type "Actor Object Reference") (OtherComp :type "PrimitiveComponent Object Reference") (OtherBodyIndex :type Integer) (bFromSweep :type Boolean) (SweepResult :type "HitResult Structure (by ref)"))
  ; CodigoAntigo
)

(event `OpenDoor`
  (if (`self.canOpen`)
    (bind (_direction _alpha) (`Timeline|Timeline Door`)
      (:`Update`
        (`SceneComponent.K2_SetWorldRotation` (`self.Door`) (`KismetMathLibrary.MakeRotator` 0.0 0.0 (`KismetMathLibrary.Lerp` 0.0 90.0 _alpha)) false false))
      (:`Finished`
        (`self.LevelChange`)))))

(fn `NewFunction`)

(fn `UserConstructionScript`)