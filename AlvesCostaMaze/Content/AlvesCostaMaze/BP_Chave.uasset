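; BP_Chave is the key pickup in a maze game that lets the player unlock the exit door.
; On BeginPlay it caches the first BP_Door found in the level.
; When BP_PlayerPawn overlaps its trigger box, it reports the pickup to BP_GameMode and checks whether Keys equals one.
; If so, it updates the pawn's Venceu win flag, on a win prints congratulations and sets the door's CanOpen, then destroys itself.
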(event OnComponentBeginOverlap(TriggerBox)
  (params (OverlappedComponent :type Primitive%20Component%20Object%20Reference) (OtherActor :type Actor%20Object%20Reference) (OtherComp :type Primitive%20Component%20Object%20Reference) (OtherBodyIndex :type Integer) (bFromSweep :type Boolean) (SweepResult :type Hit%20Result%20Structure%20%28by%20ref%29))
  (bind _asbp_player_pawn (Utilities|Casting|CastToBP_PlayerPawn OtherActor))
  (bind _asbp_game_mode (Utilities|Casting|CastToBP_GameMode (Game|GetGameMode)))
  (Default|PlayerPegouaAchave _asbp_game_mode _asbp_player_pawn)
  (if (== (Variables|/Game/AlvesCostaMaze/GameMode/BP_GameMode.BP_GameMode_C|GetKeys _asbp_game_mode) 1)
    (Variables|/Game/AlvesCostaMaze/BP_PlayerPawn.BP_PlayerPawn_C|SetbVenceu? _asbp_player_pawn (>= (stale _result) 1.0))
    (if (Variables|/Game/AlvesCostaMaze/BP_PlayerPawn.BP_PlayerPawn_C|GetbVenceu? _asbp_player_pawn)
      (Development|PrintString "Parabens voce venceu")
      (Variables|/Game/AlvesCostaMaze/BP_Door.BP_Door_C|SetcanOpen (Variables|Default|GetDoor) true))
    (Actor|DestroyActor)))

(event EventBeginPlay
  (bind _outactors (Actor|GetAllActorsOfClass "/Game/AlvesCostaMaze/BP_Door.BP_Door_C"))
  (bind _asbp_door (Utilities|Casting|CastToBP_Door (Utilities|Array|Get(acopy) _outactors)))
  (Variables|Default|SetDoor _asbp_door))

(event Collision|EventActorBeginOverlap
  (params (OtherActor :type Actor%20Object%20Reference)))

(event EventTick
  (params (DeltaSeconds :type Float%20%28single-precision%29)))

(fn ConstructionScript)